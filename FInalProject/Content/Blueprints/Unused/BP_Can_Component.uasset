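; Component for a held can item that throws it back into the world as a pickup; it sits in the Unused folder.
; DropObject spawns BP_Can_Pickup at a camera-rotated offset from the player pawn and pushes its mesh along the view direction with a mass-independent force.
; It then clears HasItem on BP_FirstPersonCharacter and destroys itself.
; The event graph holds no active logic.
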(fn `DropObject`
  (bind _returnvalue (`PlayerCameraManager.GetCameraRotation` (`GameplayStatics.GetPlayerCameraManager` 0)))
  ;[1 1 1] CHANGE THIS TO CORRECT PICKUP BP
  (bind _returnvalue_2 (`|SpawnActorFromClass` "/Game/Blueprints/Unused/BP_Can_Pickup.BP_Can_Pickup_C" (`KismetMathLibrary.MakeTransform` (+ (`Actor.K2_GetActorLocation` (`GameplayStatics.GetPlayerPawn` 0)) (`KismetMathLibrary.GreaterGreater_VectorRotator` (`self.ProjectileOffset`) _returnvalue)) _returnvalue) "Undefined" "OverrideRootScale" null null))
  (`self.AddForce` (`StaticMeshActor.StaticMeshComponent` _returnvalue_2) (* (`KismetMathLibrary.GreaterGreater_VectorRotator` (1.0 0.0 0.0) _returnvalue) 100000.0) "None" true)
  (bind _asbp_first_person_character (cast `/Game/Blueprints/BP_FirstPersonCharacter` (`GameplayStatics.GetPlayerPawn` 0)))
  (set `/Game/Blueprints/BP_FirstPersonCharacter.HasItem` false _asbp_first_person_character)
  (`self.K2_DestroyComponent`))