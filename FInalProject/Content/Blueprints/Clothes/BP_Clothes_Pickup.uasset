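; BP_Clothes_Pickup is a clothing pickup that dresses the first-person character when overlapped.
; On overlap it checks the character's HasItem flag, and if unset it adds a clothes component to the player, sets the flag and destroys itself.
; The new component copies the pickup's static mesh and first material, despite the function being named ChangeSkeletalMesh.
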(event `self.ReceiveActorBeginOverlap`
  (params (OtherActor :type "Actor Object Reference"))
  (bind _asbp_first_person_character (cast `/Game/Blueprints/BP_FirstPersonCharacter` OtherActor)
    (:`then`
      (set `self.Player` _asbp_first_person_character)
      (if (not (`/Game/Blueprints/BP_FirstPersonCharacter.HasItem` _asbp_first_person_character))
        (`self.ChangeSkeletalMesh`)
        (set `/Game/Blueprints/BP_FirstPersonCharacter.HasItem` true _asbp_first_person_character)
        (`self.K2_DestroyActor`)))
    (:`CastFailed`
      (`KismetSystemLibrary.PrintString` "Cast to BP_FirstPersonCharacter FAILED"))))

(fn `ChangeSkeletalMesh`
  (bind _staticmeshcomponent (`self.StaticMeshComponent`))
  (bind _returnvalue (`AddComponent|NODE_AddBP_Clothes_Test-0` :`self` (`self.Player`)))
  (`StaticMeshComponent.SetStaticMesh` _returnvalue (`StaticMeshComponent.StaticMesh` _staticmeshcomponent))
  (`PrimitiveComponent.SetMaterial` _returnvalue 0 (`PrimitiveComponent.GetMaterial` _staticmeshcomponent 0)))

(fn `UserConstructionScript`)