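; BP_Clothes_Component is the held form of a clothing item on the first-person character.
; On BeginPlay it snaps to the first-person mesh's GripPoint socket and adds the IMC_Weapons input mapping.
; IA_Drop spawns a BP_Clothes_Pickup ahead of the camera, copies over the mesh and first material, and throws it along the view direction.
; It then clears the player's HasItem flag and destroys itself.
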(event `self.ReceiveBeginPlay`
  (bind _asbp_first_person_character (cast `/Game/Blueprints/BP_FirstPersonCharacter` (`self.GetOwner`)))
  (bind _output_get (set `self.First Person Character` _asbp_first_person_character))
  (`self.K2_AttachToComponent` (`/Game/Blueprints/BP_FirstPersonCharacter.FirstPersonMesh` _output_get) "GripPoint" "SnapToTarget" "SnapToTarget" "SnapToTarget")
  (bind _asplayer_controller (cast `PlayerController` (`Pawn.GetController` (`self.First Person Character`))))
  (bind _returnvalue (pcsubsystem `EnhancedInputLocalPlayerSubsystem` _asplayer_controller))
  (`/Engine/EditorBlueprintResources/StandardMacros.IsValid` _returnvalue
    (:`Is Valid`
      (`EnhancedInputSubsystemInterface.AddMappingContext` _returnvalue "/Game/FirstPerson/Input/IMC_Weapons.IMC_Weapons" 1 (struct)))))

(event `EnhancedInput|/Game/FirstPerson/Input/Actions/IA_Drop`
  (params (ActionValue :type Boolean) (ElapsedSeconds :type "Float (double-precision)") (TriggeredSeconds :type "Float (double-precision)") (InputAction :type "InputAction Object Reference" :default "/Game/FirstPerson/Input/Actions/IA_Drop.IA_Drop"))
  (:`Triggered`
    (`self.DropObject`)))

(fn `DropObject`
  (bind _returnvalue (`PlayerCameraManager.GetCameraRotation` (`GameplayStatics.GetPlayerCameraManager` 0)))
  ;[1 1 1] CHANGE THIS TO CORRECT PICKUP BP
  (bind _returnvalue_2 (`|SpawnActorFromClass` "/Game/Blueprints/Clothes/BP_Clothes_Pickup.BP_Clothes_Pickup_C" (`KismetMathLibrary.MakeTransform` (+ (`Actor.K2_GetActorLocation` (`GameplayStatics.GetPlayerPawn` 0)) (`KismetMathLibrary.GreaterGreater_VectorRotator` (`self.ProjectileOffset`) _returnvalue)) _returnvalue) "Undefined" "OverrideRootScale" null null))
  (bind _staticmeshcomponent (`StaticMeshActor.StaticMeshComponent` _returnvalue_2))
  (`self.SetStaticMesh` _staticmeshcomponent (`self.StaticMesh`))
  (`self.SetMaterial` _staticmeshcomponent 0 (`self.GetMaterial` 0))
  (`self.AddForce` (`StaticMeshActor.StaticMeshComponent` _returnvalue_2) (* (`KismetMathLibrary.GreaterGreater_VectorRotator` (1.0 0.0 0.0) _returnvalue) 100000.0) "None" true)
  (bind _asbp_first_person_character (cast `/Game/Blueprints/BP_FirstPersonCharacter` (`GameplayStatics.GetPlayerPawn` 0)))
  (set `/Game/Blueprints/BP_FirstPersonCharacter.HasItem` false _asbp_first_person_character)
  (`self.K2_DestroyComponent`))