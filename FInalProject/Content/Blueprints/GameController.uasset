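; GameController sits on the first-person character and runs the cleanup game loop, including HUD or tutorial setup, pause menu and win/lose screens.
; A Delay on Tick updates meters about once per second unless paused: addiction rises unless the player sits, and amplifies stress gain.
; Maxed stress means losing.
; Winning requires removing clothes and garbage up to targets set from placed pickup counts minus one, with garbage's target able to grow.
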(event `self.ReceiveBeginPlay`
  (bind _returnvalue (`GameplayStatics.GetPlayerController` 0))
  (bind _returnvalue_2 (`GameplayStatics.GetPlayerController` 0))
  (bind _asbp_first_person_character (cast `/Game/Blueprints/BP_FirstPersonCharacter` (`self.GetOwner` self)))
  (set `self.Player` _asbp_first_person_character)
  (bind _outactors (`GameplayStatics.GetAllActorsOfClass` "/Game/Blueprints/Clothes/BP_Clothes_Pickup.BP_Clothes_Pickup_C"))
  (set `self.ClothesMax` (`KismetArrayLibrary.Array_Length` _outactors))
  (set `self.Clothes` 0)
  (bind _outactors_2 (`GameplayStatics.GetAllActorsOfClass` "/Game/Blueprints/Garbage/BP_Garbage_Pickup.BP_Garbage_Pickup_C"))
  (set `self.GarbageMax` (`KismetArrayLibrary.Array_Length` _outactors_2))
  (`/Engine/EditorBlueprintResources/StandardMacros.DecrementInt` (`self.ClothesMax`)
    (:`  `
      (`/Engine/EditorBlueprintResources/StandardMacros.DecrementInt` (`self.GarbageMax`)
        (:`  `
          (set `self.Garbage` 0)
          (set `self.StressLevel` 0.0)
          (set `self.AddictionLevel` 0.0)
          (if (`self.Tutorial`)
            (bind _returnvalue_3 (`|CreateWidget` "/Game/UI/Tutorial_WBP.Tutorial_WBP_C"))
            (`UserWidget.AddToViewport` _returnvalue_3 0)
            (set `PlayerController.bShowMouseCursor` false _returnvalue_2)
            (`WidgetBlueprintLibrary.SetInputMode_GameAndUIEx` _returnvalue_2 _returnvalue_3)
            (`GameplayStatics.SetGamePaused` false)
            (else
              (bind _returnvalue_4 (`|CreateWidget` "/Game/UI/MyHUD_WBP.MyHUD_WBP_C"))
              (`UserWidget.AddToViewport` _returnvalue_4 0)
              (set `PlayerController.bShowMouseCursor` false _returnvalue)
              (`WidgetBlueprintLibrary.SetInputMode_GameOnly` _returnvalue))))))))

(event `self.ReceiveTick`
  (params (DeltaSeconds :type "Float (single-precision)"))
  (`KismetSystemLibrary.Delay` 1.0)
  (if (not (`GameplayStatics.IsGamePaused`))
    (`self.AdjustStress`)
    (`self.AdjustAddiction`)))

(event `Key|P`
  (params (Key :type "Key Structure"))
  (bind _returnvalue (`GameplayStatics.GetPlayerController` 0))
  (:`Pressed`
    (`GameplayStatics.SetGamePaused` true)
    (bind _returnvalue_2 (`|CreateWidget` "/Game/UI/PauseMenu_WBP.PauseMenu_WBP_C"))
    (`UserWidget.AddToViewport` _returnvalue_2 0)
    (set `PlayerController.bShowMouseCursor` true _returnvalue)
    (`WidgetBlueprintLibrary.SetInputMode_GameOnly` _returnvalue)))

(fn `AddGarbageMax`
  (`/Engine/EditorBlueprintResources/StandardMacros.IncrementInt` (`self.GarbageMax`)))

(fn `AdjustAddiction`
  (bind _addictionlevel (`self.AddictionLevel`))
  (bind _addictionrate (`self.AddictionRate`))
  (if (`/Game/Blueprints/BP_FirstPersonCharacter.IsSitting` (`self.Player`))
    (bind _output_get (set `self.AddictionLevel` (- _addictionlevel (* _addictionrate (`self.AddictionReductionMultiplier`)))))
    (if (<= _output_get 0.0)
      (set `self.AddictionLevel` 0.0))
    (else
      (bind _output_get_2 (set `self.AddictionLevel` (+ _addictionlevel _addictionrate)))
      (if (>= _output_get_2 100)
        (set `self.AddictionLevel` (`self.MaxAddiction`))))))

(fn `AdjustStress`
  (bind _returnvalue (`GameplayStatics.GetPlayerController` 0))
  (bind _output_get (set `self.StressLevel` (+ (`self.StressLevel`) (`self.StressRate`) (* (`KismetMathLibrary.SafeDivide` (`self.AddictionLevel`) (`self.MaxAddiction`)) 2.0 (`self.StressRate`)))))
  (if (>= _output_get (`self.MaxStress`))
    (bind _returnvalue_2 (`|CreateWidget` "/Game/UI/YouLose.YouLose_C"))
    (`UserWidget.AddToViewport` _returnvalue_2 0)
    (`GameplayStatics.SetGamePaused` true)
    (`WidgetBlueprintLibrary.SetInputMode_UIOnlyEx` _returnvalue null)
    (set `PlayerController.bShowMouseCursor` true _returnvalue)))

(fn `Check for Win`
  (bind _returnvalue (`GameplayStatics.GetPlayerController` 0))
  (bind _returnvalue_2 (`GameplayStatics.GetPlayerController` 0))
  (if (and (`self.ClothesDone`) (`self.GarbageDone`))
    (if (`self.Tutorial`)
      (bind _returnvalue_3 (`|CreateWidget` "/Game/UI/TutorialFinish.TutorialFinish_C"))
      (`UserWidget.AddToViewport` _returnvalue_3 0)
      (`GameplayStatics.SetGamePaused` true)
      (`WidgetBlueprintLibrary.SetInputMode_UIOnlyEx` _returnvalue null)
      (set `PlayerController.bShowMouseCursor` true _returnvalue)
      (else
        (bind _returnvalue_4 (`|CreateWidget` "/Game/UI/YouWin.YouWin_C"))
        (`UserWidget.AddToViewport` _returnvalue_4 0)
        (`GameplayStatics.SetGamePaused` true)
        (`WidgetBlueprintLibrary.SetInputMode_UIOnlyEx` _returnvalue_2 null)
        (set `PlayerController.bShowMouseCursor` true _returnvalue_2)))))

(fn `ClothesRemoved`
  (bind _result (`/Engine/EditorBlueprintResources/StandardMacros.IncrementInt` (`self.Clothes`))
    (:`  `
      (if (>= _result (`self.ClothesMax`))
        (set `self.ClothesDone` true)
        (`self.Check for Win`)))))

(fn `GarbageRemoved`
  (bind _result (`/Engine/EditorBlueprintResources/StandardMacros.IncrementInt` (`self.Garbage`))
    (:`  `
      (if (>= _result (`self.GarbageMax`))
        (set `self.GarbageDone` true)
        (`self.Check for Win`)))))